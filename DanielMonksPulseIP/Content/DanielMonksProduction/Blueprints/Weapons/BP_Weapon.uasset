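; BP_Weapon is a hitscan weapon whose stats drive fire rate, pellet count, range, spread and damage, with a shrink gun variant.
; Shoot is gated by CanShoot and a FireDelay timer, then runs one debug-drawn Visibility line trace per bullet, offset by a random BulletDeviance vector.
; Hits apply damage, then either scale down movable actors for the shrink gun or push physics-simulating components with a damage-scaled impulse.
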(event `ShootTimerExpired`
  ; Only let the gun shoot if its timer is expired, determined by rate of fire in the shoot function
  (set `self.CanShoot` true))

(fn `BulletDeviance`
  (returns (BulletDeviance :type "Vector Structure"))
  (bind _bulletaccuracy (`self.BulletAccuracy`))
  (bind _bulletaccuracy_2 (`self.BulletAccuracy`))
  (bind _bulletaccuracy_3 (`self.BulletAccuracy`))
  ; Multiply gun bullet accuracy by -1 for minimum value, use default value for maximum value. Do this three times to make a vector and set that as bullet deviance.
  (return (`KismetMathLibrary.MakeVector` (`KismetMathLibrary.RandomFloatInRange` (* _bulletaccuracy_2 -1.0) _bulletaccuracy_2) (`KismetMathLibrary.RandomFloatInRange` (* _bulletaccuracy_3 -1.0) _bulletaccuracy_3) (`KismetMathLibrary.RandomFloatInRange` (* _bulletaccuracy -1.0) _bulletaccuracy))))

(fn `Shoot`
  (params (`Origins Location` :type "Vector Structure") (`Forward Vector` :type "Vector Structure"))
  ; Check if the weapon can shoot
  (if (`self.CanShoot`)
    (set `self.CanShoot` false)
    ; Set if the weapon can shoot timer by rate of fire
    (`KismetSystemLibrary.K2_SetTimerDelegate` (`|CreateDelegate` :!event `ShootTimerExpired`) (`self.FireDelay`))
    ; Perform for each bullet the gun can shoot
    (for _ (range 1 (+ (`self.BulletAmount`) 1))
      ; Standard line trace code. Added bullet deviance function for bullet accuracy.
      (bind _outhit (`KismetSystemLibrary.LineTraceSingle` :`Start` `Origins Location` :`End` (+ `Origins Location` (* `Forward Vector` (`self.Range`)) (`self.BulletDeviance`)) :`TraceChannel` "TraceTypeQuery1" :`DrawDebugType` "ForDuration" :`DrawTime` 1.0))
      ; If target is valid, apply damage
      (`/Engine/EditorBlueprintResources/StandardMacros.IsValid` (`.HitComponent` (`GameplayStatics.BreakHitResult` _outhit))
        (:`Is Valid`
          (`GameplayStatics.ApplyDamage` (`.HitActor` (`GameplayStatics.BreakHitResult` _outhit)) (`self.Damage`))
          ; Check if the gun is the shrink cannon
          (if (`self.IsShrinkGun`)
            (bind _returnvalue (`|EnumEquality` (`SceneComponent.Mobility` (`.HitComponent` (`GameplayStatics.BreakHitResult` _outhit))) "Movable"))
            ; If shrink gun, get the actor's 3D scale then multiply it by the gun's shrink amount (0.9)
            (if _returnvalue
              (`self.SetActorScale3D` (`.HitActor` (`GameplayStatics.BreakHitResult` _outhit)) (* (`self.GetActorScale3D` (`.HitActor` (`GameplayStatics.BreakHitResult` _outhit))) (`self.ShrinkAmount`))))
            (else
              ; Apply impulse based on gun damage
              (if (and (`SceneComponent.IsSimulatingPhysics` (`.HitComponent` (`GameplayStatics.BreakHitResult` _outhit)) "None") _returnvalue)
                (`PrimitiveComponent.AddImpulseAtLocation` (`.HitComponent` (`GameplayStatics.BreakHitResult` _outhit)) (* `Forward Vector` (`self.Damage`)) (`.Location` (`GameplayStatics.BreakHitResult` _outhit)) "None")))))))))

(fn `UserConstructionScript`)