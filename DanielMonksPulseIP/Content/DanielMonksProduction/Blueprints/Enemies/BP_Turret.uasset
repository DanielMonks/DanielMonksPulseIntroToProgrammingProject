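; BP_Turret is an enemy turret that tracks and shoots the player on sight, and is destroyed when its health component runs out.
; Each PawnSensing sighting turns it toward the player, then fires the child-actor gun from BulletStart.
; TargetPlayer interpolates rotation, yawing the whole actor while pitching only the head within a clamped range.
; A flag and delay, advanced by further sightings, throttle the alarm sound.
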(event `self.ReceiveBeginPlay`
  ; Sets BP_TurretGun as the gun component of the turret
  (bind _asbp_turret_gun (cast `/Game/DanielMonksProduction/Blueprints/Weapons/BP_TurretGun` (`ChildActorComponent.ChildActor` (`self.Gun`))))
  (set `self.GunBP` _asbp_turret_gun))

(event `self.PawnSensing.OnSeePawn`
  (params (Pawn :type "Pawn Object Reference"))
  (bind _bulletstart (`self.BulletStart`))
  ; On detecting the player, the target player function is ran and the player is shot at
  (bind _asbp_first_person_shooter_character (cast `/Game/DanielMonksProduction/Blueprints/BP_FirstPersonShooterCharacter` Pawn))
  (`self.TargetPlayer` _asbp_first_person_shooter_character)
  (`/Game/DanielMonksProduction/Blueprints/Weapons/BP_Weapon.Shoot` (`self.GunBP`) (`SceneComponent.K2_GetComponentLocation` _bulletstart) (`SceneComponent.GetForwardVector` _bulletstart))
  ; Checks if the alarm sound is playing before replaying it and ensures it can't be played over itself
  (if (`self.AlarmPlaying`)
    (`KismetSystemLibrary.Delay` 1.0)
    (set `self.AlarmPlaying` false)
    (else
      (`GameplayStatics.PlaySoundAtLocation` "/Game/DanielMonksProduction/Sounds/Turret_Alarm.Turret_Alarm" (`self.K2_GetActorLocation`) (struct) 1.0 1.0 0.0 null null null null)
      (set `self.AlarmPlaying` true))))

(event `self.BPC_Health.OnHealthDepleted`
  ; Turret destroyed on health depleted
  (`self.K2_DestroyActor`))

(fn `TargetPlayer`
  (params (Player :type "Actor Object Reference"))
  (bind _head (`self.Head`))
  (bind (_returnvalue_roll _returnvalue_pitch _returnvalue_yaw) (`KismetMathLibrary.BreakRotator` (`KismetMathLibrary.RInterpTo` (`SceneComponent.K2_GetComponentRotation` _head) (`KismetMathLibrary.FindLookAtRotation` (`SceneComponent.K2_GetComponentLocation` _head) (`self.K2_GetActorLocation` Player)) (`GameplayStatics.GetWorldDeltaSeconds`) (`self.RotationSpeed`))))
  ; Gets player location and the current location of the head of the turret before having it move to face the player
  ; Y value is clamped to prevent turret head going too far up or down
  (`SceneComponent.K2_SetRelativeRotation` (`self.Head`) (`KismetMathLibrary.MakeRotator` 0.0 (`KismetMathLibrary.FClamp` _returnvalue_pitch -20.0 20.0)) false false)
  (`self.K2_SetActorRotation` (`KismetMathLibrary.MakeRotator` 0.0 0.0 _returnvalue_yaw)))

(fn `UserConstructionScript`)