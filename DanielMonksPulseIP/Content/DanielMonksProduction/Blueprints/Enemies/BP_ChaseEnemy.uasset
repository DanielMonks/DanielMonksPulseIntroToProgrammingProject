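; BP_ChaseEnemy is a suicide enemy that patrols around its spawn point and chases the player it spots, exploding on contact for damage.
; PawnSensing starts the chase with an alarm sound, and a delayed self-calling event rechecks distance, resuming patrol once the player escapes.
; Patrol loops through AIMoveTo to random navigable points, using a wider radius after the first sighting.
; BPC_Health destroys it when health depletes.
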(event `RepeatPatrol`
  ; Check if original location has been set
  (if (`self.OriginalLocationSet`) :!label _label
    ; Check if the player has been detected previously
    (if (`self.HasSeenPlayer`)
      ; If the player has been detected before, the enemy is alerted and patrols a larger area near its original location
      (bind _randomlocation (`NavigationSystemV1.K2_GetRandomLocationInNavigableRadius` (`self.OriginalLocation`) (`KismetMathLibrary.FClamp` (`KismetMathLibrary.RandomFloat`) 2000.0 5000.0) null null))
      (`|AIMoveTo` self _randomlocation null
        (:`OnSuccess`
          ; Moves to a new location upon completing its movement
          (`self.RepeatPatrol`)))
      (else
        ; If the player has not been detected, the enemy isn't alerted and patrols a small area near its original location
        (bind _randomlocation_2 (`NavigationSystemV1.K2_GetRandomLocationInNavigableRadius` (`self.OriginalLocation`) (`KismetMathLibrary.FClamp` (`KismetMathLibrary.RandomFloat`) 1000.0 2000.0) null null))
        (`|AIMoveTo` self _randomlocation_2 null
          (:`OnSuccess`
            (`self.RepeatPatrol`)))))
    (else
      ; Sets original location before having the enemy patrol
      (set `self.OriginalLocation` (`self.K2_GetActorLocation`))
      (set `self.OriginalLocationSet` true)
      (`self.RepeatPatrol`))))

(event `self.ReceiveBeginPlay`
  ; Check if original location has been set
  (goto _label))

(event `PlayerEscaped`
  ; Set the player as having been seen on first detection, making the enemy alert from then onwards. We also rerun the loop from here if the player has escaped.
  (bind _asbp_first_person_shooter_character (cast `/Game/DanielMonksProduction/Blueprints/BP_FirstPersonShooterCharacter` (stale `self.PawnSensing.OnSeePawn` Pawn) :!label _label_2))
  ; Check the current range of the player from the enemy
  (if (<= (`self.GetDistanceTo` _asbp_first_person_shooter_character) 3000.0)
    ; If the player is in range, the enemy chases them. We check if the alarm is playing to make sure it sounds play over itself. Every 5 seconds we rerun the loop to check if the player has escaped, in which case the enemy goes back to patrol, this time on high alert.
    (`|AIMoveTo` self (0.0 0.0 0.0) _asbp_first_person_shooter_character
      (:`then`
        (if (`self.AlarmPlaying`)
          (`KismetSystemLibrary.Delay` 5.0)
          (set `self.AlarmPlaying` false)
          (`self.PlayerEscaped`)
          (else
            (`GameplayStatics.PlaySoundAtLocation` "/Game/DanielMonksProduction/Sounds/Enemy_Alarm.Enemy_Alarm" (`self.K2_GetActorLocation`) (struct) 1.0 1.0 0.0 null null null null)
            (set `self.AlarmPlaying` true)
            (`KismetSystemLibrary.Delay` 5.0)
            (`self.PlayerEscaped`))))
      (:`OnSuccess`
        ; If the enemy makes contact with the player, they explode, dealing damage and playing an explosion sound effect
        (bind _asbp_first_person_shooter_character_2 (cast `/Game/DanielMonksProduction/Blueprints/BP_FirstPersonShooterCharacter` (`GameplayStatics.GetPlayerCharacter` 0)))
        (`GameplayStatics.ApplyDamage` _asbp_first_person_shooter_character_2 40.0)
        (`self.K2_DestroyActor`)
        (`GameplayStatics.PlaySoundAtLocation` "/Game/DanielMonksProduction/Sounds/Enemy_Explosion.Enemy_Explosion" (`self.K2_GetActorLocation`) (struct) 1.0 1.0 0.0 null null null null)))
    (else
      ; If the player gets far enough away, the enemy returns to patrolling
      (`self.RepeatPatrol`))))

(event `self.PawnSensing.OnSeePawn`
  (params (Pawn :type "Pawn Object Reference"))
  ; Set the player as having been seen on first detection, making the enemy alert from then onwards. We also rerun the loop from here if the player has escaped.
  (set `self.HasSeenPlayer` true)
  (goto _label_2))

(event `self.BPC_Health.OnHealthDepleted`
  ; Destroyed on health depleted
  (`self.K2_DestroyActor`))

(fn `UserConstructionScript`)