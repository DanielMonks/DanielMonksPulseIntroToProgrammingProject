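; Objective actor that completes when its referenced platform is powered.
; On BeginPlay it checks that PlatformRef is valid and binds OnDoorUnlocked to that platform's PowerThePlatform event.
; When the event fires, it calls Completed and destroys itself, with no tick or overlap logic of its own.
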(event `self.ReceiveBeginPlay`
  (bind _platformref (`self.PlatformRef`))
  (`parent.ReceiveBeginPlay`)
  (`/Engine/EditorBlueprintResources/StandardMacros.IsValid` _platformref
    (:`Is Valid`
      (add `/Game/DanielMonksProduction/Blueprints/LevelComponents/MovingPlatforms/BP_MovingPlatformEnergyPowered.PowerThePlatform` _platformref (delegate `OnDoorUnlocked`)))))

(event `OnDoorUnlocked`
  (`self.Completed`)
  (`self.K2_DestroyActor`))

(fn `UserConstructionScript`
  (`parent.UserConstructionScript`))