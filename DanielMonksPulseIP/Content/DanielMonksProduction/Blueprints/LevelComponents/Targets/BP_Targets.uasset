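; Shooting target actor that cycles between green, yellow and orange and awards score by its colour when destroyed.
; BeginPlay picks a random starting state, then Tick steps the colour through timed delays, gated by a loop-complete flag.
; When BPC_Health depletes, it turns grey, stops its InterpToMovement, adds that colour's points to BP_FirstPersonShooterCharacter's PlayerScore with printed feedback, and hides its lights.
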(event `self.ReceiveBeginPlay`
  ; Set random material initially for target variety
  (set `self.TargetMaterial` (`KismetMathLibrary.RandomIntegerInRange` 1 3)))

(event `self.ReceiveTick`
  (params (DeltaSeconds :type "Float (single-precision)"))
  ; Check the targets every tick. Loop only runs if not hit and loop is complete
  (if (`self.HasBeenHit`)
    _
    (elif (`self.LoopIsComplete`)
      (set `self.LoopIsComplete` false)
      ; If the target is orange, set to green and complete loop after 2 seconds
      (if (== (`self.TargetMaterial`) 3)
        (`PrimitiveComponent.SetMaterial` (`self.Cylinder`) 0 "/Game/DanielMonksProduction/Materials/MAT_Green.MAT_Green")
        (set `self.TargetMaterial` 1)
        (`KismetSystemLibrary.Delay` 2.0)
        (set `self.LoopIsComplete` true)
        (else
          ; If target is green, set to yellow and complete loop after 3 seconds
          (if (== (`self.TargetMaterial`) 1)
            (`PrimitiveComponent.SetMaterial` (`self.Cylinder`) 0 "/Game/DanielMonksProduction/Materials/MAT_Yellow.MAT_Yellow")
            (set `self.TargetMaterial` 2)
            (`KismetSystemLibrary.Delay` 3.0)
            (set `self.LoopIsComplete` true)
            (else
              ; If target is yellow, set to orange and complete loop after 4 seconds
              (if (== (`self.TargetMaterial`) 2)
                (`PrimitiveComponent.SetMaterial` (`self.Cylinder`) 0 "/Game/DanielMonksProduction/Materials/MAT_Orange.MAT_Orange")
                (set `self.TargetMaterial` 3)
                (`KismetSystemLibrary.Delay` 4.0)
                (set `self.LoopIsComplete` true)))))))))

(event `self.BPC_Health.OnHealthDepleted`
  ; Once the target's health is depleted, check the current material and only run if the target hasn't been hit before
  (if (== (`self.TargetMaterial`) 1)
    (if (not (`self.HasBeenHit`))
      ; Make target grey to show it's been hit
      (`PrimitiveComponent.SetMaterial` (`self.Cylinder`) 0 "/Game/DanielMonksProduction/Materials/MAT_Grey.MAT_Grey")
      ; Set target to hit so loop is closed, stop target moving
      (set `self.HasBeenHit` true)
      (`ActorComponent.SetComponentTickEnabled` (`self.InterpToMovement`) false)
      ; Call appropriate score event
      (`self.SetScoreGreenTarget` null)
      ; Disable Lights
      (`SceneComponent.SetVisibility` (`self.FrontLight`) false false :!label _label)
      (`SceneComponent.SetVisibility` (`self.BackLight`) false false))
    (elif (== (`self.TargetMaterial`) 2)
      (if (not (`self.HasBeenHit`))
        (`PrimitiveComponent.SetMaterial` (`self.Cylinder`) 0 "/Game/DanielMonksProduction/Materials/MAT_Grey.MAT_Grey")
        (set `self.HasBeenHit` true)
        (`ActorComponent.SetComponentTickEnabled` (`self.InterpToMovement`) false)
        (`self.SetScoreYellowTarget` null)
        (goto _label))
      (elif (== (`self.TargetMaterial`) 3)
        (if (not (`self.HasBeenHit`))
          (`PrimitiveComponent.SetMaterial` (`self.Cylinder`) 0 "/Game/DanielMonksProduction/Materials/MAT_Grey.MAT_Grey")
          (set `self.HasBeenHit` true)
          (`ActorComponent.SetComponentTickEnabled` (`self.InterpToMovement`) false)
          (`self.SetScoreOrangeTarget` null)
          (goto _label))))))

(event `SetScoreGreenTarget`
  (params (SelfActor :type "Actor Object Reference") (OtherActor :type "Actor Object Reference") (NormalImpulse :type "Vector Structure") (Hit :type "HitResult Structure (by ref)"))
  ; If the target was green, we cast to the player blueprint to add 50 to the score and print the result for the player
  (bind _asbp_first_person_shooter_character (cast `/Game/DanielMonksProduction/Blueprints/BP_FirstPersonShooterCharacter` (`GameplayStatics.GetPlayerCharacter` 0)))
  (bind _output_get (set `/Game/DanielMonksProduction/Blueprints/BP_FirstPersonShooterCharacter.PlayerScore` (+ (`/Game/DanielMonksProduction/Blueprints/BP_FirstPersonShooterCharacter.PlayerScore` _asbp_first_person_shooter_character) 50) _asbp_first_person_shooter_character))
  (`KismetSystemLibrary.PrintString` (`KismetStringLibrary.Conv_IntToString` _output_get))
  (`KismetSystemLibrary.PrintString` "Total Score:")
  (`KismetSystemLibrary.PrintString` "Green target hit! +50 to score"))

(event `SetScoreYellowTarget`
  (params (SelfActor :type "Actor Object Reference") (OtherActor :type "Actor Object Reference") (NormalImpulse :type "Vector Structure") (Hit :type "HitResult Structure (by ref)"))
  ; If the target was yellow, we cast to the player blueprint to add 20 to the score and print the result for the player
  (bind _asbp_first_person_shooter_character (cast `/Game/DanielMonksProduction/Blueprints/BP_FirstPersonShooterCharacter` (`GameplayStatics.GetPlayerCharacter` 0)))
  (bind _output_get (set `/Game/DanielMonksProduction/Blueprints/BP_FirstPersonShooterCharacter.PlayerScore` (+ (`/Game/DanielMonksProduction/Blueprints/BP_FirstPersonShooterCharacter.PlayerScore` _asbp_first_person_shooter_character) 20) _asbp_first_person_shooter_character))
  (`KismetSystemLibrary.PrintString` (`KismetStringLibrary.Conv_IntToString` _output_get))
  (`KismetSystemLibrary.PrintString` "Total Score:")
  (`KismetSystemLibrary.PrintString` "Yellow target hit! +20 to score"))

(event `SetScoreOrangeTarget`
  (params (SelfActor :type "Actor Object Reference") (OtherActor :type "Actor Object Reference") (NormalImpulse :type "Vector Structure") (Hit :type "HitResult Structure (by ref)"))
  ; If the target was orange, we cast to the player blueprint to add 10 to the score and print the result for the player
  (bind _asbp_first_person_shooter_character (cast `/Game/DanielMonksProduction/Blueprints/BP_FirstPersonShooterCharacter` (`GameplayStatics.GetPlayerCharacter` 0)))
  (bind _output_get (set `/Game/DanielMonksProduction/Blueprints/BP_FirstPersonShooterCharacter.PlayerScore` (+ (`/Game/DanielMonksProduction/Blueprints/BP_FirstPersonShooterCharacter.PlayerScore` _asbp_first_person_shooter_character) 10) _asbp_first_person_shooter_character))
  (`KismetSystemLibrary.PrintString` (`KismetStringLibrary.Conv_IntToString` _output_get))
  (`KismetSystemLibrary.PrintString` "Total Score:")
  (`KismetSystemLibrary.PrintString` "Orange target hit! +10 to score"))

(fn `UserConstructionScript`)