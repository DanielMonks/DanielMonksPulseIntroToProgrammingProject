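; BP_Door is an interactable swinging door that can be locked until it is unlocked.
; Interact toggles between Open and Close, and Open only works while the door is not locked.
; A Timeline drives the mesh's relative yaw from 0 to 110 degrees, and Close reverses it.
; Unlock clears the lock and opens the door immediately, intended for key pickup.
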(event `Open`
  ; Check if the door is locked, if it's not then set it to opened
  (if (not (`self.Locked`))
    (set `self.Opened` true)
    ; Create movement over a period of time when the door is opened
    (bind (_direction _doorrotation) (`Timeline|Timeline` :!label _label)
      (:`Update`
        (`SceneComponent.K2_SetRelativeRotation` (`self.Mesh`) (`KismetMathLibrary.MakeRotator` 0.0 0.0 (`KismetMathLibrary.Lerp` 0.0 110.0 _doorrotation)) false false)))))

(event `Close`
  ; Reverse the door's movement when closed and set it as closed
  (set `self.Opened` false)
  (goto _label :!via `Reverse`))

(event `Unlock`
  ; Unlock the door once the key is picked up
  (set `self.Locked` false)
  (`self.Open`))

(event `Interact`
  ; Check if the door is open or closed before having it swing open or shut on player interaction
  (if (`self.Opened`)
    (`self.Close`)
    (else
      (`self.Open`))))

(fn `UserConstructionScript`)