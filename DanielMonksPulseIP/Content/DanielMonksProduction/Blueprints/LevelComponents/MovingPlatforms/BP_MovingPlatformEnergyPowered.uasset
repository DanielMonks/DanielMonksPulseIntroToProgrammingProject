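; BP_MovingPlatformEnergyPowered is a moving platform that only travels while its energy component holds charge.
; BeginPlay disables ticking on the InterpToMovement component, and Tick re-enables it whenever BPCEnergy has energy above zero.
; A 15-second Delay inside Tick paces each EnergyDecreased call, and movement ticking switches off again when energy reaches zero.
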(event `self.ReceiveBeginPlay`
  ; When the game starts, the platform waits to move
  (`ActorComponent.SetComponentTickEnabled` (`self.InterpToMovement`) false))

(event `self.ReceiveTick`
  (params (DeltaSeconds :type "Float (single-precision)"))
  (bind _bpc_energy (`self.BPC_Energy`))
  ; The platform checks itself for energy every tick. If it has energy, it will move.
  (if (> (`/Game/DanielMonksProduction/Blueprints/Components/BPC_Energy.Energy` (`self.BPC_Energy`)) 0.0)
    (`ActorComponent.SetComponentTickEnabled` (`self.InterpToMovement`) true)
    ; Every minute that passes the platform loses energy. Once it reaches 0 it will stop moving.
    (`KismetSystemLibrary.Delay` 15.0)
    (`/Game/DanielMonksProduction/Blueprints/Components/BPC_Energy.EnergyDecreased` _bpc_energy)
    (if (== (`/Game/DanielMonksProduction/Blueprints/Components/BPC_Energy.Energy` _bpc_energy) 0.0)
      (`ActorComponent.SetComponentTickEnabled` (`self.InterpToMovement`) false))))

(event `self.ReceiveActorBeginOverlap`
  (params (OtherActor :type "Actor Object Reference")))

(fn `UserConstructionScript`)