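; Energy component that tracks an Energy value and moves it one unit at a time between empty and a fixed maximum of five.
; EnergyIncreased and EnergyDecreased check their limit, adjust the value, print debug text and broadcast OnEnergyChanged, always passing zero.
; EnergyDecreased also broadcasts OnEnergyDepleted on reaching zero, though its debug message wrongly reads "Energy Increased".
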(event `EnergyIncreased`
  ; Check if energy is at maximum value before increasing it
  (if (== (`self.Energy`) 5.0)
    (`KismetSystemLibrary.PrintString` "Maximum energy reached. Energy cannot be exchanged.")
    (else
      ; Increase energy and give the new energy level
      (bind _output_get (set `self.Energy` (+ (`self.Energy`) 1.0)))
      (`KismetSystemLibrary.PrintString` (`KismetStringLibrary.Concat_StrStr` (`KismetSystemLibrary.GetDisplayName` self) "Energy Increased. Current Energy Level: " (`KismetStringLibrary.Conv_DoubleToString` _output_get)))
      (`self.OnEnergyChanged` 0.0))))

(event `EnergyDecreased`
  ; Check if energy is at 0 before decreasing
  (if (== (`self.Energy`) 0.0)
    (`KismetSystemLibrary.PrintString` "Energy is depleted and cannot be exchanged.")
    (else
      ; Decrease energy and give the new level, call energy depleted in case this needs to be checked
      (bind _output_get (set `self.Energy` (- (`self.Energy`) 1.0)))
      (`KismetSystemLibrary.PrintString` (`KismetStringLibrary.Concat_StrStr` (`KismetSystemLibrary.GetDisplayName` self) "Energy Increased. Current Energy Level: " (`KismetStringLibrary.Conv_DoubleToString` _output_get)))
      (`self.OnEnergyChanged` 0.0)
      (if (== (`self.Energy`) 0.0)
        (`self.OnEnergyDepleted`)))))